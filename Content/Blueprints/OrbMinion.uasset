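; Orb minion actor, built on a parent AI base, that appears to be an air summon of the top-down player character.
; Each tick it updates animation and, once dead, clears the player's AirSpawned flag and destroys itself.
; The animation event shows an idle flipbook on death, otherwise tracks last move direction, though every direction and movement state uses the same Character_idle flipbook.
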(event EventBeginPlay
  (|CallParentFunction) ; This node is disabled and will not be called.\nDrag off pins to build functionality.
)

(event Collision|EventActorBeginOverlap
  (params (OtherActor :type Actor%20Object%20Reference))
  (|CallParentFunction OtherActor) ; This node is disabled and will not be called.\nDrag off pins to build functionality.
)

(event EventTick
  (params (DeltaSeconds :type Float%20%28single-precision%29))
  (CallFunction|UpdateAnimation)
  (if (Variables|Default|GetDeadAIBase)
    (bind _asbp_top_down_character (Utilities|Casting|CastToBP_TopDownCharacter (Game|GetPlayerCharacter 0)))
    (Variables|/Game/ThirdPersonBP/Blueprints/BP_TopDownCharacter.BP_TopDownCharacter_C|SetAirSpawned _asbp_top_down_character false)
    (Actor|DestroyActor)))

(event EventAnimationStateMachine
  (params (IsDead? :type Boolean))
  ;[1 1 1] Animation
  (if IsDead?
    (Sprite|SetFlipbook (Variables|Default|GetSprite) "/Game/Sprites/FB_Idle.FB_Idle")
    (else
      (if (or (!= (Input|AxisValues|GetMoveForward) 0.0) (!= (Input|AxisValues|GetMoveRight) 0.0))
        (Variables|Default|SetLastMoveDirection (select (> (Input|AxisValues|GetMoveForward) 0.0) "NewEnumerator0" (select (< (Input|AxisValues|GetMoveForward) 0.0) "NewEnumerator1" (select (> (Input|AxisValues|GetMoveRight) 0.0) "NewEnumerator3" "NewEnumerator2")))))
      (Sprite|SetFlipbook (Variables|Default|GetSprite) (select (> (Math|Vector|VectorLength (Transformation|GetVelocity)) 0.0) (Utilities|Select :Index (Variables|Default|GetLastMoveDirection) :NewEnumerator0 "/Game/Summoner/Flipbooks/character_idle.character_idle" :NewEnumerator1 "/Game/Summoner/Flipbooks/character_idle.character_idle" :NewEnumerator2 "/Game/Summoner/Flipbooks/character_idle.character_idle" :NewEnumerator3 "/Game/Summoner/Flipbooks/character_idle.character_idle") (Utilities|Select :Index (Variables|Default|GetLastMoveDirection) :NewEnumerator0 "/Game/Summoner/Flipbooks/character_idle.character_idle" :NewEnumerator1 "/Game/Summoner/Flipbooks/character_idle.character_idle" :NewEnumerator2 "/Game/Summoner/Flipbooks/character_idle.character_idle" :NewEnumerator3 "/Game/Summoner/Flipbooks/character_idle.character_idle"))))))

(fn ConstructionScript
  (|CallParentFunction))