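; Base 2D summon character that follows the player on the X/Z plane, snapping back when they leave its detection sphere.
; Tick drives movement and directional flipbooks, and destroys it once damage brings health to exactly zero.
; The sphere records Enemy-tagged targets but never sets HasTarget true, so the chase branch stays unreached here.
; A weapon box starts a half-second repeating damage loop on overlapping enemies.
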(event OnComponentBeginOverlap(Sphere)
  (params (OverlappedComponent :type Primitive%20Component%20Object%20Reference) (OtherActor :type Actor%20Object%20Reference) (OtherComp :type Primitive%20Component%20Object%20Reference) (OtherBodyIndex :type Integer) (bFromSweep :type Boolean) (SweepResult :type Hit%20Result%20Structure%20%28by%20ref%29))
  ;[1 1 1] Detection
  (if (Actor|ActorHasTag OtherActor "Enemy")
    (if (not (Variables|Default|GetHasTarget))
      (Variables|Default|SetTarget OtherActor)
      (Variables|Default|SetHasTarget false))))

(event OnComponentEndOverlap(Sphere)
  (params (OverlappedComponent :type Primitive%20Component%20Object%20Reference) (OtherActor :type Actor%20Object%20Reference) (OtherComp :type Primitive%20Component%20Object%20Reference) (OtherBodyIndex :type Integer))
  ;[1 1 1] Detection
  (Utilities|Casting|CastToBP_TopDownCharacter OtherActor)
  (Variables|Default|SetIsOverlapping false))

(event OnComponentBeginOverlap(Box1)
  (params (OverlappedComponent :type Primitive%20Component%20Object%20Reference) (OtherActor :type Actor%20Object%20Reference) (OtherComp :type Primitive%20Component%20Object%20Reference) (OtherBodyIndex :type Integer) (bFromSweep :type Boolean) (SweepResult :type Hit%20Result%20Structure%20%28by%20ref%29))
  ;[1 1 1] Detection
  (if (Actor|ActorHasTag OtherActor "Enemy")
    (Variables|Default|SetIsOverlappingWeapon true)
    (if (Variables|Default|GetSpecialAttack)
      _
      (else
        _))
    (Utilities|FlowControl|DoOnce false :!label _label
      (:Completed
        (Variables|Default|SetAttacking true)
        (Utilities|FlowControl|Delay 0.5 :!label _label_2)
        (if (not (Variables|Default|GetDeadAIBase))
          (if (Variables|Default|GetHit)
            (goto _label_2)
            (elif (Variables|Default|GetIsOverlappingWeapon)
              (bind _asbase_ai (Utilities|Casting|CastToBaseAi OtherActor))
              (Default|DamageSystem _asbase_ai 1.0)
              (goto _label_2)
              (else
                (Variables|Default|SetAttacking false)
                (goto _label Reset)))))))))

(event OnComponentEndOverlap(Box1)
  (params (OverlappedComponent :type Primitive%20Component%20Object%20Reference) (OtherActor :type Actor%20Object%20Reference) (OtherComp :type Primitive%20Component%20Object%20Reference) (OtherBodyIndex :type Integer))
  ;[1 1 1] Detection
  (if (Actor|ActorHasTag OtherActor "Enemy")
    (Variables|Default|SetIsOverlappingWeapon false)))

(event Custom|MoveToCharacter
  (bind _capsulecomponent (Variables|Collision|GetCapsuleComponent))
  (bind _capsulecomponent_2 (Variables|Collision|GetCapsuleComponent))
  (bind _returnvalue (Transformation|GetWorldLocation _capsulecomponent_2))
  (bind _returnvalue_2 (Transformation|GetWorldLocation _capsulecomponent))
  ;[1 1 1] AI Movement
  (if (Variables|Default|GetHasTarget)
    (bind _asbase_ai (Utilities|Casting|CastToBaseAi (Variables|Default|GetTarget)))
    (if (>= (- (.x (Transformation|GetWorldLocation (Variables|/Script/Engine.Character|GetCapsuleComponent _asbase_ai))) (.x _returnvalue)) 0.0)
      (Variables|Default|SetISMovingRight true)
      (else
        (Variables|Default|SetISMovingRight false)))
    (Pawn|Input|AddMovementInput "1.000000, 0, 0" (- (.x (Transformation|GetWorldLocation (Variables|/Script/Engine.Character|GetCapsuleComponent _asbase_ai))) (.x _returnvalue)) false)
    (if (>= (- (.z (Transformation|GetWorldLocation (Variables|/Script/Engine.Character|GetCapsuleComponent _asbase_ai))) (.z _returnvalue)) 0.0)
      (Variables|Default|SetIsMovingUp true)
      (Variables|Default|SetIsMovingDown false)
      (else
        (Variables|Default|SetIsMovingDown true)
        (Variables|Default|SetIsMovingUp false)))
    (Pawn|Input|AddMovementInput "0.000000,0.000000,1.000000" (- (.z (Transformation|GetWorldLocation (Variables|/Script/Engine.Character|GetCapsuleComponent _asbase_ai))) (.z _returnvalue)) false)
    (elif (Variables|Default|GetIsOverlapping)
      (bind _asbp_top_down_character (Utilities|Casting|CastToBP_TopDownCharacter (Game|GetPlayerCharacter 0)))
      (if (>= (- (.x (Transformation|GetWorldLocation (Variables|/Script/Engine.Character|GetCapsuleComponent _asbp_top_down_character))) (.x _returnvalue_2)) 0.0)
        (Variables|Default|SetISMovingRight true)
        (else
          (Variables|Default|SetISMovingRight false)))
      (Pawn|Input|AddMovementInput "1.000000, 0, 0" (- (.x (Transformation|GetWorldLocation (Variables|/Script/Engine.Character|GetCapsuleComponent _asbp_top_down_character))) (.x _returnvalue_2)) false)
      (if (>= (- (.z (Transformation|GetWorldLocation (Variables|/Script/Engine.Character|GetCapsuleComponent _asbp_top_down_character))) (.z _returnvalue_2)) 0.0)
        (Variables|Default|SetIsMovingUp true)
        (Variables|Default|SetIsMovingDown false)
        (else
          (Variables|Default|SetIsMovingDown true)
          (Variables|Default|SetIsMovingUp false)))
      (Pawn|Input|AddMovementInput "0.000000,0.000000,1.000000" (- (.z (Transformation|GetWorldLocation (Variables|/Script/Engine.Character|GetCapsuleComponent _asbp_top_down_character))) (.z _returnvalue_2)) false)
      (else
        (bind _asbp_top_down_character_2 (Utilities|Casting|CastToBP_TopDownCharacter (Game|GetPlayerCharacter 0)))
        (Transformation|SetActorLocation (Math|Vector|MakeVector (.x (Transformation|GetWorldLocation (Variables|/Script/Engine.Character|GetCapsuleComponent _asbp_top_down_character_2))) (.y (Transformation|GetWorldLocation (Variables|/Script/Engine.Character|GetCapsuleComponent _asbp_top_down_character_2))) (- (.z (Transformation|GetWorldLocation (Variables|/Script/Engine.Character|GetCapsuleComponent _asbp_top_down_character_2))) 5.0)) false false)
        (Variables|Default|SetIsOverlapping true)
        (Variables|Default|SetHasTarget false)))))

(event Custom|Health%20System
  (params (HealthOut :type Float%20%28single-precision%29))
  ;[1 1 1] Handle Health & Damage
  (bind _output_get (Variables|Default|SetCharHealth (+ (Variables|Default|GetCharHealth) HealthOut)))
  (Math|Float|CompareFloat _output_get 1.0
    (:>
      (Variables|Default|SetCharHealth 1.0))))

(event Custom|UpdateAnimation
  ;[1 1 1] Handle Animation
  (if (Variables|Default|GetDeadAIBase)
    (Sprite|SetFlipbook (Variables|Default|GetSprite) "/Game/Sprites/FB_Idle.FB_Idle")
    (else
      (CallFunction|MovetoCharacter)
      (if (or (!= (Input|AxisValues|GetMoveForward) 0.0) (!= (Input|AxisValues|GetMoveRight) 0.0))
        (Variables|Default|SetLastMoveDirection (select (> (Input|AxisValues|GetMoveForward) 0.0) "NewEnumerator0" (select (< (Input|AxisValues|GetMoveForward) 0.0) "NewEnumerator1" (select (> (Input|AxisValues|GetMoveRight) 0.0) "NewEnumerator3" "NewEnumerator2")))))
      (Sprite|SetFlipbook (Variables|Default|GetSprite) (select (> (Math|Vector|VectorLength (Transformation|GetVelocity)) 0.0) (Utilities|Select :Index (Variables|Default|GetLastMoveDirection) :NewEnumerator0 "/Game/Sprites/FB_RunUp.FB_RunUp" :NewEnumerator1 "/Game/Sprites/FB_RunDown.FB_RunDown" :NewEnumerator2 "/Game/Sprites/FB_RunLeft.FB_RunLeft" :NewEnumerator3 "/Game/Sprites/FB_RunUp.FB_RunUp") (Utilities|Select :Index (Variables|Default|GetLastMoveDirection) :NewEnumerator0 "/Game/Sprites/FB_Idle.FB_Idle" :NewEnumerator1 "/Game/Sprites/FB_Idle.FB_Idle" :NewEnumerator2 "/Game/Sprites/FB_Idle.FB_Idle" :NewEnumerator3 "/Game/Sprites/FB_Idle.FB_Idle"))))))

(event Custom|DamageSystem
  (params (DmgOut :type Float%20%28single-precision%29))
  ;[1 1 1] Handle Health & Damage
  (Audio|PlaySoundatLocation 0 "0, 0, 0" "0, 0, 0" 1.0 1.0 0.0 0 0 0)
  (bind _output_get (Variables|Default|SetCharHealth (- (Variables|Default|GetCharHealth) DmgOut)))
  (Math|Float|CompareFloat _output_get 0.0
    (:>
      (Development|PrintText "alive"))
    (:==
      (Variables|Default|SetDeadAIBase true))))

(event Custom|CommandAttack
  ;[1 1 1] Detection
)

(event Custom|Lives%20System
  (params (Lives%20Out :type Integer)))

(event Collision|EventActorBeginOverlap
  (params (OtherActor :type Actor%20Object%20Reference)))

(event EventTick
  (params (DeltaSeconds :type Float%20%28single-precision%29))
  ;[1 1 1] Tick - Updates animation
  (CallFunction|UpdateAnimation)
  (if (Variables|Default|GetDeadAIBase)
    (Actor|DestroyActor)))

(fn ConstructionScript)

(fn AnimationStateMachine
  (params (IsDead? :type Boolean))
  (if IsDead?
    (Sprite|SetFlipbook (Variables|Default|GetSprite) "/Game/Sprites/FB_Idle.FB_Idle")
    (else
      (if (or (!= (Input|AxisValues|GetMoveForward) 0.0) (!= (Input|AxisValues|GetMoveRight) 0.0))
        (Variables|Default|SetLastMoveDirection (select (> (Input|AxisValues|GetMoveForward) 0.0) "NewEnumerator0" (select (< (Input|AxisValues|GetMoveForward) 0.0) "NewEnumerator1" (select (> (Input|AxisValues|GetMoveRight) 0.0) "NewEnumerator3" "NewEnumerator2")))))
      (Sprite|SetFlipbook (Variables|Default|GetSprite) (select (> (Math|Vector|VectorLength (Transformation|GetVelocity)) 0.0) (Utilities|Select :Index (Variables|Default|GetLastMoveDirection) :NewEnumerator0 "/Game/Sprites/FB_RunUp.FB_RunUp" :NewEnumerator1 "/Game/Sprites/FB_RunDown.FB_RunDown" :NewEnumerator2 "/Game/Sprites/FB_RunLeft.FB_RunLeft" :NewEnumerator3 "/Game/Sprites/FB_RunUp.FB_RunUp") (Utilities|Select :Index (Variables|Default|GetLastMoveDirection) :NewEnumerator0 "/Game/Sprites/FB_Idle.FB_Idle" :NewEnumerator1 "/Game/Sprites/FB_Idle.FB_Idle" :NewEnumerator2 "/Game/Sprites/FB_Idle.FB_Idle" :NewEnumerator3 "/Game/Sprites/FB_Idle.FB_Idle"))))))