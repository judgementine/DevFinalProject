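; RockMinion is a Paper2D top-down minion character that follows the player.
; Each tick it steers along X and Y toward the player and picks a directional flipbook from movement input and velocity.
; Health events heal up to a cap or apply damage, flagging death only at exactly zero, which idles and stops the sprite.
; Enemy overlaps set attack flags, but the damage call is unwired.
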(event OnComponentBeginOverlap(Sphere)
  (params (OverlappedComponent :type Primitive%20Component%20Object%20Reference) (OtherActor :type Actor%20Object%20Reference) (OtherComp :type Primitive%20Component%20Object%20Reference) (OtherBodyIndex :type Integer) (bFromSweep :type Boolean) (SweepResult :type Hit%20Result%20Structure%20%28by%20ref%29))
  (if (Actor|ActorHasTag OtherActor "Player")
    (Utilities|Casting|CastToBP_TopDownCharacter OtherActor)
    (Variables|Default|SetIsOverlapping true)
    (elif (Actor|ActorHasTag OtherActor "Enemy")
      (Utilities|Array|Add (Variables|Default|GetActorArray) OtherActor))))

(event OnComponentEndOverlap(Sphere)
  (params (OverlappedComponent :type Primitive%20Component%20Object%20Reference) (OtherActor :type Actor%20Object%20Reference) (OtherComp :type Primitive%20Component%20Object%20Reference) (OtherBodyIndex :type Integer))
  (Utilities|Casting|CastToBP_TopDownCharacter OtherActor)
  (Variables|Default|SetIsOverlapping false))

(event OnComponentBeginOverlap(Box1)
  (params (OverlappedComponent :type Primitive%20Component%20Object%20Reference) (OtherActor :type Actor%20Object%20Reference) (OtherComp :type Primitive%20Component%20Object%20Reference) (OtherBodyIndex :type Integer) (bFromSweep :type Boolean) (SweepResult :type Hit%20Result%20Structure%20%28by%20ref%29))
  (if (Actor|ActorHasTag OtherActor "Enemy")
    (Variables|Default|SetIsOverlappingWeapon true)
    (if (Variables|Default|GetSpecialAttack)
      _
      (else
        _))
    (Utilities|FlowControl|DoOnce false :!label _label
      (:Completed
        (Variables|Default|SetAttacking true)
        (Utilities|FlowControl|Delay 0.5 :!label _label_2)
        (if (not (Variables|Default|GetDeadAIBase))
          (if (Variables|Default|GetHit)
            (goto _label_2)
            (elif (not (Variables|Default|GetIsOverlappingWeapon))
              (Variables|Default|SetAttacking false)
              (goto _label))))))))

(event Custom|MoveToCharacter
  (bind _capsulecomponent (Variables|Collision|GetCapsuleComponent))
  (bind _returnvalue (Transformation|GetWorldLocation _capsulecomponent))
  (if (Variables|Default|GetisAttacking)
    _
    (else
      _))
  (bind _asbp_top_down_character (Utilities|Casting|CastToBP_TopDownCharacter (Game|GetPlayerCharacter 0)))
  (if (>= (- (.x (Transformation|GetWorldLocation (Variables|/Script/Engine.Character|GetCapsuleComponent _asbp_top_down_character))) (.x _returnvalue)) 0.0)
    (Variables|Default|SetISMovingRight true)
    (else
      (Variables|Default|SetISMovingRight false)))
  (Pawn|Input|AddMovementInput "1.000000, 0, 0" (- (.x (Transformation|GetWorldLocation (Variables|/Script/Engine.Character|GetCapsuleComponent _asbp_top_down_character))) (.x _returnvalue)) false)
  (Development|PrintString "MinionMoving")
  (if (>= (- (.y (Transformation|GetWorldLocation (Variables|/Script/Engine.Character|GetCapsuleComponent _asbp_top_down_character))) (.y _returnvalue)) 0.0)
    (Variables|Default|SetIsMovingUp true)
    (Variables|Default|SetIsMovingDown false)
    (else
      (Variables|Default|SetIsMovingDown true)
      (Variables|Default|SetIsMovingUp false)))
  (Pawn|Input|AddMovementInput "0.000000,1.000000,0.000000" (- (.y (Transformation|GetWorldLocation (Variables|/Script/Engine.Character|GetCapsuleComponent _asbp_top_down_character))) (.y _returnvalue)) false))

(event Custom|Health%20System
  (params (HealthOut :type Float%20%28single-precision%29))
  ;[1 1 1] Handle Health & Damage
  (bind _output_get (Variables|Default|SetCharHealth (+ (Variables|Default|GetCharHealth) HealthOut)))
  (Math|Float|CompareFloat _output_get 1.0
    (:>
      (Variables|Default|SetCharHealth 1.0))))

(event Custom|UpdateAnimation
  ;[1 1 1] Handle Animation
  (if (Variables|Default|GetDeadAIBase)
    (Sprite|SetFlipbook (Variables|Default|GetSprite) "/Game/Sprites/FB_Idle.FB_Idle")
    (else
      (CallFunction|MovetoCharacter)
      (if (or (!= (Input|AxisValues|GetMoveForward) 0.0) (!= (Input|AxisValues|GetMoveRight) 0.0))
        (Variables|Default|SetLastMoveDirection (select (> (Input|AxisValues|GetMoveForward) 0.0) "NewEnumerator0" (select (< (Input|AxisValues|GetMoveForward) 0.0) "NewEnumerator1" (select (> (Input|AxisValues|GetMoveRight) 0.0) "NewEnumerator3" "NewEnumerator2")))))
      (Sprite|SetFlipbook (Variables|Default|GetSprite) (select (> (Math|Vector|VectorLength (Transformation|GetVelocity)) 0.0) (Utilities|Select :Index (Variables|Default|GetLastMoveDirection) :NewEnumerator0 "/Game/Sprites/FB_RunUp.FB_RunUp" :NewEnumerator1 "/Game/Sprites/FB_RunDown.FB_RunDown" :NewEnumerator2 "/Game/Sprites/FB_RunLeft.FB_RunLeft" :NewEnumerator3 "/Game/Sprites/FB_RunUp.FB_RunUp") (Utilities|Select :Index (Variables|Default|GetLastMoveDirection) :NewEnumerator0 "/Game/Sprites/FB_Idle.FB_Idle" :NewEnumerator1 "/Game/Sprites/FB_Idle.FB_Idle" :NewEnumerator2 "/Game/Sprites/FB_Idle.FB_Idle" :NewEnumerator3 "/Game/Sprites/FB_Idle.FB_Idle"))))))

(event Custom|DamageSystem
  (params (DmgOut :type Float%20%28single-precision%29))
  ;[1 1 1] Handle Health & Damage
  (Audio|PlaySoundatLocation 0 "0, 0, 0" "0, 0, 0" 1.0 1.0 0.0 0 0 0)
  (bind _output_get (Variables|Default|SetCharHealth (- (Variables|Default|GetCharHealth) DmgOut)))
  (Math|Float|CompareFloat _output_get 0.0
    (:>
      (Development|PrintText "alive"))
    (:==
      (Variables|Default|SetDeadAIBase true))))

(event Custom|CommandAttack)

(event Custom|Lives%20System
  (params (Lives%20Out :type Integer)))

(event Collision|EventActorBeginOverlap
  (params (OtherActor :type Actor%20Object%20Reference)))

(event EventTick
  (params (DeltaSeconds :type Float%20%28single-precision%29))
  ;[1 1 1] Tick - Updates animation
  (CallFunction|UpdateAnimation)
  (if (Variables|Default|GetDeadAIBase)
    (Audio|Components|Audio|Stop (Variables|Default|GetSprite))))

(event EventBeginPlay
  ;[1 1 1] Handle UI
)

(event Input|AxisEvents|InputAxisMoveForward
  (params (AxisValue :type Float%20%28single-precision%29))
  (Pawn|Input|AddMovementInput "0,1.000000, 0" AxisValue false))

(event Input|AxisEvents|InputAxisMoveRight
  (params (AxisValue :type Float%20%28single-precision%29))
  (Pawn|Input|AddMovementInput "1.000000, 0, 0" AxisValue false))

(fn ConstructionScript)

(fn AnimationStateMachine
  (params (IsDead? :type Boolean))
  (if IsDead?
    (Sprite|SetFlipbook (Variables|Default|GetSprite) "/Game/Sprites/FB_Idle.FB_Idle")
    (else
      (if (or (!= (Input|AxisValues|GetMoveForward) 0.0) (!= (Input|AxisValues|GetMoveRight) 0.0))
        (Variables|Default|SetLastMoveDirection (select (> (Input|AxisValues|GetMoveForward) 0.0) "NewEnumerator0" (select (< (Input|AxisValues|GetMoveForward) 0.0) "NewEnumerator1" (select (> (Input|AxisValues|GetMoveRight) 0.0) "NewEnumerator3" "NewEnumerator2")))))
      (Sprite|SetFlipbook (Variables|Default|GetSprite) (select (> (Math|Vector|VectorLength (Transformation|GetVelocity)) 0.0) (Utilities|Select :Index (Variables|Default|GetLastMoveDirection) :NewEnumerator0 "/Game/Sprites/FB_RunUp.FB_RunUp" :NewEnumerator1 "/Game/Sprites/FB_RunDown.FB_RunDown" :NewEnumerator2 "/Game/Sprites/FB_RunLeft.FB_RunLeft" :NewEnumerator3 "/Game/Sprites/FB_RunUp.FB_RunUp") (Utilities|Select :Index (Variables|Default|GetLastMoveDirection) :NewEnumerator0 "/Game/Sprites/FB_Idle.FB_Idle" :NewEnumerator1 "/Game/Sprites/FB_Idle.FB_Idle" :NewEnumerator2 "/Game/Sprites/FB_Idle.FB_Idle" :NewEnumerator3 "/Game/Sprites/FB_Idle.FB_Idle"))))))